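; BP_CollisionHands provides physics-driven left and right hands that follow a pair of motion controllers.
; Setup stores the controller references and has each Physics Handle grab its hand skeletal mesh at the mesh's current location and rotation.
; Every Tick, each handle's target is set to its controller's world transform, so the hands are pulled along through physics rather than attached directly.
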(event EventTick
  (params (DeltaSeconds :type Float%20%28single-precision%29))
  (bind _leftmotioncontroller (Variables|Default|GetLeftMotionController))
  (bind _rightmotioncontroller (Variables|Default|GetRightMotionController))
  (bind _returnvalue (Transformation|GetWorldTransform _rightmotioncontroller))
  (bind _returnvalue_2 (Transformation|GetWorldTransform _leftmotioncontroller))
  (Class|PhysicsHandleComponent|SetTargetLocationandRotation (Variables|Default|GetRightPhysicsHandle) (.location _returnvalue) (.rotation _returnvalue))
  (Class|PhysicsHandleComponent|SetTargetLocationandRotation (Variables|Default|GetLeftPhysicsHandle) (.location _returnvalue_2) (.rotation _returnvalue_2)))

(fn ConstructionScript)

(fn Setup
  (params (LeftMotionController :type Motion%20Controller%20Component%20Object%20Reference) (RightMotionController :type Motion%20Controller%20Component%20Object%20Reference))
  (bind _righthandskeletalmesh (Variables|Default|GetRightHandSkeletalMesh))
  (bind _lefthandskeletalmesh (Variables|Default|GetLeftHandSkeletalMesh))
  (bind _returnvalue (Transformation|GetWorldTransform _lefthandskeletalmesh))
  (bind _returnvalue_2 (Transformation|GetWorldTransform _righthandskeletalmesh))
  (Utilities|FlowControl|Sequence
    (:then_0
      (Variables|Default|SetLeftMotionController LeftMotionController)
      (Physics|Components|PhysicsHandle|GrabComponentatLocationwithRotation (Variables|Default|GetLeftPhysicsHandle) _lefthandskeletalmesh "None" (.location _returnvalue) (.rotation _returnvalue)))
    (:then_1
      (Variables|Default|SetRightMotionController RightMotionController)
      (Physics|Components|PhysicsHandle|GrabComponentatLocationwithRotation (Variables|Default|GetRightPhysicsHandle) _righthandskeletalmesh "None" (.location _returnvalue_2) (.rotation _returnvalue_2)))))